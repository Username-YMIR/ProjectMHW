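; Base long sword weapon Blueprint, currently holding only prototype hit detection.
; When the HitBox begins an overlap, it fires a short Visibility line trace from the box along its forward vector, with timed debug drawing.
; It prints the name of the actor the trace hits, which may differ from the overlapped actor, and applies no damage.
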(event `self.HitBox.OnComponentBeginOverlap`
  (params (OverlappedComponent :type "PrimitiveComponent Object Reference") (OtherActor :type "Actor Object Reference") (OtherComp :type "PrimitiveComponent Object Reference") (OtherBodyIndex :type Integer) (bFromSweep :type Boolean) (SweepResult :type "HitResult Structure (by ref)"))
  (bind _hitbox (`self.HitBox`))
  (bind _returnvalue (`SceneComponent.K2_GetComponentLocation` _hitbox))
  (bind _outhit (`KismetSystemLibrary.LineTraceSingle` :`Start` _returnvalue :`End` (+ _returnvalue (* (`SceneComponent.GetForwardVector` _hitbox) 200.0)) :`TraceChannel` "TraceTypeQuery1" :`DrawDebugType` "ForDuration"))
  (`KismetSystemLibrary.PrintString` (`KismetSystemLibrary.GetDisplayName` (`.HitActor` (`GameplayStatics.BreakHitResult` _outhit)))))

(fn `UserConstructionScript`)