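; Glavenus monster tail actor that drops under physics when spawned and then settles into a fixed pose, apparently as the severed tail.
; On BeginPlay the Tail becomes physics-only, ignores world and pawn channels, and gets a downward impulse.
; After a short delay, a vertical trace finds the surface; on a hit, the actor snaps to an offset below it, rotates to a set pose keeping its yaw, and stops simulating.
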(event `self.ReceiveBeginPlay`
  (bind _returnvalue (`self.K2_GetActorLocation`))
  (bind _tail (`self.Tail`))
  (`PrimitiveComponent.SetCollisionEnabled` _tail "PhysicsOnly")
  (`PrimitiveComponent.SetCollisionResponseToChannel` _tail "ECC_WorldStatic" "ECR_Ignore")
  (`PrimitiveComponent.SetCollisionResponseToChannel` _tail "ECC_WorldDynamic" "ECR_Ignore")
  (`PrimitiveComponent.SetCollisionResponseToChannel` _tail "ECC_Pawn" "ECR_Ignore")
  (`PrimitiveComponent.SetSimulatePhysics` _tail true)
  (`PrimitiveComponent.AddImpulse` _tail (0.0 0.0 -300.0) "None" false)
  (`KismetSystemLibrary.Delay` 0.8)
  (bind (_outhit _returnvalue_2) (`KismetSystemLibrary.LineTraceSingle` :`Start` (+ _returnvalue (`KismetMathLibrary.MakeVector` 0.0 0.0 100.0)) :`End` (+ _returnvalue (`KismetMathLibrary.MakeVector` 0.0 0.0 -500.0)) :`TraceChannel` "TraceTypeQuery1" :`DrawDebugType` "ForDuration"))
  (if _returnvalue_2
    (`self.K2_SetActorLocation` (+ (`.ImpactPoint` (`GameplayStatics.BreakHitResult` _outhit)) (`KismetMathLibrary.MakeVector` 0.0 0.0 -700.0)))
    (`self.K2_SetActorRotation` (`KismetMathLibrary.MakeRotator` 90.0 90.0 (.yaw (`self.K2_GetActorRotation`))))
    (`PrimitiveComponent.SetSimulatePhysics` _tail false)))

(fn `UserConstructionScript`)