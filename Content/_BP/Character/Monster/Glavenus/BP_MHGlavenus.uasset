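; Glavenus monster Blueprint that adds groggy and phase 2 reactions plus a severable tail.
; Groggy plays a montage, while phase 2 plays a tail-heating montage and finishes the transition however it ends.
; Accepted hits whose closest bone is a tail bone subtract fixed damage from tail HP, with debug prints.
; At zero, a separate tail actor spawns at the tail socket and the tail is flagged severed.
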(event `self.BP_OnEnterGroggy`
  (params (GroggyIndex :type Integer))
  (`|PlayMontage` null "/Game/Assets/Monster/Dinovald/Animation/2/Glavenus_Grrogys_Montage.Glavenus_Grrogys_Montage"))

(event `self.BP_OnEnterPhase2`
  (`|PlayMontage` (`self.Mesh`) "/Game/Assets/Monster/Dinovald/Animation/Attack/Glavenus_HeatingTails_Montage.Glavenus_HeatingTails_Montage"
    (:`OnCompleted`
      (`self.FinishPhase2Transition`))
    (:`OnBlendOut`
      (`self.FinishPhase2Transition`))
    (:`OnInterrupted`
      (`self.FinishPhase2Transition`))))

(event `self.BP_OnMonsterDamageAccepted`
  (params (HitResult :type "HitResult Structure (by ref)") (AttackTag :type "GameplayTag Structure"))
  (bind _returnvalue (`self.IsTailBone` (`.ReturnValue` (`SkinnedMeshComponent.FindClosestBone_K2` (`self.Mesh`) (`.ImpactPoint` (`GameplayStatics.BreakHitResult` HitResult)) 0.0 false))))
  (if _returnvalue
    (if (== (`self.bTailSevered`) false)
      (set `self.TailHP` (- (`self.TailHP`) 100.0))
      (`KismetSystemLibrary.PrintString` (`KismetStringLibrary.Conv_DoubleToString` (`self.TailHP`)))
      (if (<= (`self.TailHP`) 0.0)
        (`|SpawnActorFromClass` "/Game/_BP/Character/Monster/Glavenus/BP_MHGlavenusTail.BP_MHGlavenusTail_C" (`SceneComponent.GetSocketTransform` (`self.Mesh`) "BoneFunction_145" "RTS_World") "Undefined" "MultiplyWithRoot" null null)
        (bind _output_get (set `self.bTailSevered` true))
        (`KismetSystemLibrary.PrintString` (`KismetStringLibrary.Conv_BoolToString` _output_get))))))

(event `self.ReceiveBeginPlay`
  (set `self.TailHP` (`self.MaxTailHP`)))

(fn `IsTailBone`
  (params (BoneName :type Name))
  (returns (ReturnValue :type Boolean))
  (return (or (== BoneName "BoneFunction_142") (== BoneName "BoneFunction_143") (== BoneName "BoneFunction_144") (== BoneName "BoneFunction_145") (== BoneName "BoneFunction_146") (== BoneName "BoneFunction_141"))))

(fn `UserConstructionScript`)